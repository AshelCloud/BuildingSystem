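; Base actor for placeable objects in the building system, handling the switch from placement preview to placed piece.
; On BeginPlay it caches the mesh's material, turns green and disables collision; events swap green, red or default materials.
; Placed restores the original material and collision, while GetBackMaterials looks up build material data by the object's material ID.
; Collision-check functions for floor, wall, roof, stair and interact objects are empty stubs.
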(event EventBeginPlay
  (Variables|Default|SetDefaultMaterial (Rendering|Material|GetMaterial (Variables|Default|GetStaticMesh) 0))
  (CallFunction|ChangeGreenMaterial)
  (Collision|SetCollisionEnabled (Variables|Default|GetStaticMesh) "NoCollision"))

(event EventChangeRedMaterial
  (Rendering|Material|SetMaterial (Variables|Default|GetStaticMesh) 0 "/Game/BuildingSystem/Blueprints/Materials/RedMaterial.RedMaterial"))

(event EventChangeDefaultMaterial
  (Rendering|Material|SetMaterial (Variables|Default|GetStaticMesh) 0 (Variables|Default|GetDefaultMaterial)))

(event EventDestroyObject
  (Actor|DestroyActor))

(event EventChangeGreenMaterial
  (Rendering|Material|SetMaterial (Variables|Default|GetStaticMesh) 0 "/Game/BuildingSystem/Blueprints/Materials/GreenMaterial.GreenMaterial"))

(event EventPlaced
  (Variables|Default|SetIsPlaced true)
  (Rendering|Material|SetMaterial (Variables|Default|GetStaticMesh) 0 (Variables|Default|GetDefaultMaterial))
  (Collision|SetCollisionEnabled (Variables|Default|GetStaticMesh) "QueryAndPhysics"))

(fn ConstructionScript)

(fn GetBackMaterials
  (bind (_buildmaterial _success) (CallFunction|ReadMaterialwithID (.MaterialID (Utilities|Struct|BreakBuildModel (Variables|Default|GetData)))))
  (return _buildmaterial _success))

(fn ReturnCheckFloorCollisions
  (return 0))

(fn ReturnCheckInteractObjectCollisions
  (return 0))

(fn ReturnCheckRoofCollisions
  (return 0))

(fn ReturnCheckStairCollisions
  (return 0))

(fn ReturnCheckWallCollisions
  (return 0))