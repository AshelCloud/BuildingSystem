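; BP_CraftingBox is a placeable crafting box in the building system that opens a crafting inventory UI when interacted with.
; Interact only responds once the box is placed, then uses a FlipFlop to alternate between opening and closing the widget.
; WBP_CraftingInventory is created and added to the viewport on first open, then cached in CraftingWidget for reuse.
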(event EventBeginPlay
  (|CallParentFunction) ; 지금 이 노드는 비활성 상태입니다. \n핀을 끌어서 다른 노드를 연결하면 활성화됩니다.
)

(event Collision|EventActorBeginOverlap
  (params (OtherActor :type Actor%20Object%20Reference))
  (|CallParentFunction OtherActor) ; 지금 이 노드는 비활성 상태입니다. \n핀을 끌어서 다른 노드를 연결하면 활성화됩니다.
)

(event EventTick
  (params (DeltaSeconds :type Float%20%28single-precision%29))
  (|CallParentFunction DeltaSeconds) ; 지금 이 노드는 비활성 상태입니다. \n핀을 끌어서 다른 노드를 연결하면 활성화됩니다.
)

(event EventInteract
  (if (Variables|Default|GetIsPlaced)
    (Utilities|FlowControl|FlipFlop
      (:A
        (Utilities|IsValid (Variables|Default|GetCrafting%20Widget)
          (:Is%20Valid
            (Default|Open (Variables|Default|GetCrafting%20Widget)))
          (:Is%20Not%20Valid
            (bind _returnvalue (UserInterface|CreateWidget "/Game/BuildingSystem/Blueprints/UserInterface/WBP_CraftingInventory.WBP_CraftingInventory_C"))
            (Variables|Default|SetCrafting%20Widget _returnvalue)
            (Default|Open (Variables|Default|GetCrafting%20Widget))
            (UserInterface|Viewport|AddtoViewport (Variables|Default|GetCrafting%20Widget) 0))))
      (:B
        (Default|Close (Variables|Default|GetCrafting%20Widget))))))

(fn ConstructionScript
  (|CallParentFunction))