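; Player building component that runs build and destroy modes, plus crafting, using a build menu and Enhanced Input.
; Starting a build consumes inventory materials; Tick then moves a spawned preview by per-type trace channels, snapping to the hit actor's collision points.
; A box-trace overlap check tints the preview green or red and gates placement; rotate input cycles snap points or yaw.
; Destroy mode highlights the traced actor red; destroying or cancelling refunds materials.
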(event Custom|OnClickGridItem
  ;[1 1 1] Input
  (if (Variables|Building|GetIsBuildMode)
    (Default|Close (Variables|Widgets|GetInventoryWidget))
    (Variables|위젯|SetIs%20Opened%20Inventory false)))

(event Custom|ResetBuild
  (Utilities|FlowControl|DoOnce false) ; enters at Reset
)

(event Input|EnhancedActionEvents|EnhancedInputActionIA_BuildMenu
  (params (ActionValue :type Boolean) (ElapsedSeconds :type Float%20%28double-precision%29) (TriggeredSeconds :type Float%20%28double-precision%29) (InputAction :type Input%20Action%20Object%20Reference :default "/Game/BuildingSystem/Input/IA_BuildMenu.IA_BuildMenu"))
  ;[1 1 1] Input
  (:Started
    (if (Variables|위젯|GetIs%20Opened%20Inventory)
      (Default|Close (Variables|Widgets|GetInventoryWidget))
      (Variables|위젯|SetIs%20Opened%20Inventory false)
      (else
        (bind _widgets (Default|Open (Variables|Widgets|GetInventoryWidget)))
        (Variables|위젯|SetIs%20Opened%20Inventory true)
        (for _array_element _widgets
          (EventDispatchers|BindEventtoOnClicked (Variables|/Game/BuildingSystem/Blueprints/UserInterface/WBP_BuildItem.WBP_BuildItem_C|GetButton _array_element) (delegate Custom|OnClickGridItem)))))))

(event Input|EnhancedActionEvents|EnhancedInputActionIA_Place
  (params (ActionValue :type Boolean) (ElapsedSeconds :type Float%20%28double-precision%29) (TriggeredSeconds :type Float%20%28double-precision%29) (InputAction :type Input%20Action%20Object%20Reference :default "/Game/BuildingSystem/Input/IA_Place.IA_Place"))
  ;[1 1 1] Input
  (:Started
    (if (Variables|Building|GetIsBuildMode)
      (if (Variables|Building|GetCan%20Build)
        (Build|BuildPlace))
      (elif (Variables|Building|GetIsDestroyMode)
        (Build|BuildDestroy)))))

(event Input|EnhancedActionEvents|EnhancedInputActionIA_DestroyMode
  (params (ActionValue :type Boolean) (ElapsedSeconds :type Float%20%28double-precision%29) (TriggeredSeconds :type Float%20%28double-precision%29) (InputAction :type Input%20Action%20Object%20Reference :default "/Game/BuildingSystem/Input/IA_DestroyMode.IA_DestroyMode"))
  ;[1 1 1] Input
  (:Started
    (Build|SetBuildMode false)
    (Build|SetDestroyMode true)))

(event Input|EnhancedActionEvents|EnhancedInputActionIA_PlaceRotate
  (params (ActionValue :type Float%20%28double-precision%29) (ElapsedSeconds :type Float%20%28double-precision%29) (TriggeredSeconds :type Float%20%28double-precision%29) (InputAction :type Input%20Action%20Object%20Reference :default "/Game/BuildingSystem/Input/IA_PlaceRotate.IA_PlaceRotate"))
  ;[1 1 1] Input
  (:Triggered
    (Build|RotateBuildingPrice ActionValue)))

(event EventBeginPlay
  (Initialize|Initialize))

(event EventTick
  (params (DeltaSeconds :type Float%20%28single-precision%29))
  (if (Variables|Building|GetIsBuildMode)
    (Utilities|FlowControl|Sequence
      (:then_0
        (Utilities|FlowControl|DoOnce false
          (:Completed
            (Build|CreateBuildPrice))))
      (:then_1
        (bind _transform (Build|BuildTrace))
        (bind _hit (Build|CheckforOverlap))
        (Variables|Building|SetCan%20Build (not _hit))
        (Transformation|SetActorTransform (Variables|Building|GetBuildinigPrice) _transform)
        (if (Variables|Building|GetCan%20Build)
          (Default|ChangeGreenMaterial (Variables|Building|GetBuildinigPrice))
          (else
            (Default|ChangeRedMaterial (Variables|Building|GetBuildinigPrice))))))
    (elif (Variables|Building|GetIsDestroyMode)
      (Build|DestroyTrace))))

(fn CheckMaterial
  (params (Material%20Type%20ID :type Integer))
  (bind _buildmaterial (CallFunction|ReadMaterialwithID Material%20Type%20ID))
  (LocalVariables|SetBuildMaterial _buildmaterial)
  (Utilities|FlowControl|Sequence
    (:then_0
      (bind _returnvalue (Material|CheckMaterialCount (.Material_1_Type (Utilities|Struct|BreakBuildMaterial (LocalVariables|GetBuildMaterial))) (.Material_1_Count (Utilities|Struct|BreakBuildMaterial (LocalVariables|GetBuildMaterial))) (Variables|컴포넌트|GetInventoryComp)))
      (LocalVariables|SetReturn%20Value (and (LocalVariables|GetReturn%20Value) _returnvalue)))
    (:then_1
      (bind _returnvalue_2 (Material|CheckMaterialCount (.Material_2_Type (Utilities|Struct|BreakBuildMaterial (LocalVariables|GetBuildMaterial))) (.Material_2_Count (Utilities|Struct|BreakBuildMaterial (LocalVariables|GetBuildMaterial))) (Variables|컴포넌트|GetInventoryComp)))
      (LocalVariables|SetReturn%20Value (and (LocalVariables|GetReturn%20Value) _returnvalue_2)))
    (:then_2
      (if (LocalVariables|GetReturn%20Value)
        (Material|ConsumeMaterial (Variables|컴포넌트|GetInventoryComp) (LocalVariables|GetBuildMaterial))
        (Default|UpdateHUD (Variables|컴포넌트|GetInventoryComp))
        (return (LocalVariables|GetReturn%20Value))
        (else
          (return (LocalVariables|GetReturn%20Value)))))))

(fn CheckMaterialCount
  (params (Type :type Integer) (Coiunt :type Integer) (Comp :type Inventory%20Component%20Object%20Reference))
  (bind _itemlmap (Variables|/Game/BuildingSystem/Blueprints/Components/InventoryComponent.InventoryComponent_C|GetItemlMap Comp))
  (bind (_value _returnvalue) (Utilities|Map|Find _itemlmap Type))
  (if (!= Type -1)
    (return (and _returnvalue (<= Coiunt _value)))
    (else
      (return true))))

(fn ConsumeMaterial
  (params (Comp :type Inventory%20Component%20Object%20Reference) (Build%20Material%20Data :type Build%20Material%20Structure))
  (LocalVariables|SetMaterial%20Map (Variables|/Game/BuildingSystem/Blueprints/Components/InventoryComponent.InventoryComponent_C|GetItemlMap Comp))
  (LocalVariables|SetBuildMaterial%20Data Build%20Material%20Data)
  (Utilities|FlowControl|Sequence
    (:then_0
      (if (!= (.material_1_type (LocalVariables|GetBuildMaterial%20Data)) -1)
        (Utilities|Map|Add (LocalVariables|GetMaterial%20Map) (.material_1_type (LocalVariables|GetBuildMaterial%20Data)) (- (.Value (Utilities|Map|Find (LocalVariables|GetMaterial%20Map) (.material_1_type (LocalVariables|GetBuildMaterial%20Data)))) (.material_1_count (LocalVariables|GetBuildMaterial%20Data))))))
    (:then_1
      (if (!= (.material_2_type (LocalVariables|GetBuildMaterial%20Data)) -1)
        (Utilities|Map|Add (LocalVariables|GetMaterial%20Map) (.material_2_type (LocalVariables|GetBuildMaterial%20Data)) (- (.Value (Utilities|Map|Find (LocalVariables|GetMaterial%20Map) (.material_2_type (LocalVariables|GetBuildMaterial%20Data)))) (.material_2_count (LocalVariables|GetBuildMaterial%20Data))))))
    (:then_2
      (Variables|/Game/BuildingSystem/Blueprints/Components/InventoryComponent.InventoryComponent_C|SetItemlMap Comp (LocalVariables|GetMaterial%20Map)))))

(fn GetBackMaterial
  (params (Data :type Build%20Material%20Structure))
  (bind _returnvalue (Game|GetPlayerCharacter 0))
  (bind _returnvalue_2 (Actor|GetComponentbyClass _returnvalue "/Game/BuildingSystem/Blueprints/Components/InventoryComponent.InventoryComponent_C"))
  (Utilities|IsValid _returnvalue_2
    (:Is%20Valid
      (bind _output_get (LocalVariables|SetInventory%20Comp _returnvalue_2))
      (Default|GetBackMaterial _output_get Data))))

(fn WidgetInitialize
  ;[1 1 1] Build Inventory 생성
  (bind _returnvalue (UserInterface|CreateWidget "/Game/BuildingSystem/Blueprints/UserInterface/WBP_BuildInventory.WBP_BuildInventory_C"))
  (bind _output_get (Variables|Widgets|SetInventoryWidget _returnvalue))
  (UserInterface|Viewport|AddtoViewport _output_get 0)
  (Widget|SetVisibility (Variables|Widgets|GetInventoryWidget) "Collapsed"))

(fn SetBuildMode
  (params (Build%20Mode :type Boolean))
  (Build|SetDestroyMode false)
  (Build|ClearBuildPrice)
  (Variables|Building|SetIsBuildMode Build%20Mode)
  (Variables|Building|SetCheckCollisionIndex 0))

(fn BuildStart
  (params (Build%20Price%20Data :type Build%20Model%20Structure))
  (bind _output_get (Variables|Building|SetBuildPriceData Build%20Price%20Data))
  (bind _success (Material|CheckMaterial (.materialid _output_get)))
  (Build|SetBuildMode _success))

(fn BuildPlace
  (Class|IPlaceableObject|Placed(Message) (Variables|Building|GetBuildinigPrice))
  (Variables|Building|SetIsBuildMode false)
  (Variables|Building|SetBuildinigPrice 0)
  (CallFunction|ResetBuild))

(fn BuildTrace
  (bind _buildinigprice (Variables|Building|GetBuildinigPrice))
  (bind _returnvalue (Transformation|GetActorTransform _buildinigprice))
  (bind _trace_type (Build|GetBuildTraceChannel))
  (bind _output_get (LocalVariables|SetIgnoreActors (Utilities|Array|MakeArray (Variables|Building|GetBuildinigPrice))))
  (bind (_start _end) (Build|GetTraceLocation))
  (bind _outhit (Collision|LineTraceByChannel _start _end _trace_type false _output_get "None"))
  (LocalVariables|SetHit%20Actor (.hitactor _outhit))
  (LocalVariables|SetHit%20Component (.hitcomponent _outhit))
  (Build|DetectCollision (LocalVariables|GetHit%20Actor))
  (if (Utilities|Array|IsValidIndex (Variables|Building|GetCheckCollisions))
    (bind (_array_element _array_index) (Utilities|Array|ForEachLoopwithBreak (Variables|Building|GetCheckCollisions) :!label _label)
      (:LoopBody
        (if (== _array_element (LocalVariables|GetHit%20Component))
          (Variables|Building|SetCheckCollisionIndex _array_index)
          (goto _label Break)))
      (:Completed
        (return (Transformation|GetWorldTransform (Utilities|Array|Get(acopy) (Variables|Building|GetCheckCollisions) (Variables|Building|GetCheckCollisionIndex))))))
    (else
      (return (Math|Transform|MakeTransform (.location _outhit) (.rotation _returnvalue) (.scale _returnvalue))))))

(fn DetectCollision
  (params (Hit%20Actor :type Actor%20Object%20Reference))
  (LocalVariables|SetHit Hit%20Actor)
  (switch Utilities|FlowControl|Switch|SwitchonModelType (.TypeID (Utilities|Struct|BreakBuildModel (Variables|Building|GetBuildPriceData)))
    (:NewEnumerator0
      (bind _collisions (Class|ISnapable|ReturnCheckFloorCollisions(Message) (LocalVariables|GetHit)))
      (Variables|Building|SetCheckCollisions _collisions))
    (:NewEnumerator1
      (bind _collisions_2 (Class|ISnapable|ReturnCheckWallCollisions(Message) (LocalVariables|GetHit)))
      (Variables|Building|SetCheckCollisions _collisions_2))
    (:NewEnumerator2
      (bind _collisions_3 (Class|ISnapable|ReturnCheckStairCollisions(Message) (LocalVariables|GetHit)))
      (Variables|Building|SetCheckCollisions _collisions_3))
    (:NewEnumerator3
      (bind _collisions_4 (Class|ISnapable|ReturnCheckRoofCollisions(Message) (LocalVariables|GetHit)))
      (Variables|Building|SetCheckCollisions _collisions_4))
    (:NewEnumerator4
      (bind _collisions_5 (Class|ISnapable|ReturnCheckInteractObjectCollisions(Message) (LocalVariables|GetHit)))
      (Variables|Building|SetCheckCollisions _collisions_5))))

(fn DestroyTrace
  (bind (_start _end) (Build|GetTraceLocation))
  (bind _outhit (Collision|LineTraceByChannel _start _end "TraceTypeQuery1" false 0 "None"))
  (if (!= (.hitactor _outhit) (Variables|Building|GetDestroy%20Actor))
    (Class|IPlaceableObject|ChangeDefaultMaterial(Message) (Variables|Building|GetDestroy%20Actor))
    (Variables|Building|SetDestroy%20Actor (.hitactor _outhit))
    (Class|IPlaceableObject|ChangeRedMaterial(Message) (Variables|Building|GetDestroy%20Actor))))

(fn BuildDestroy
  (bind _material_data (Class|IPlaceableObject|GetBackMaterials(Message) (Variables|Building|GetDestroy%20Actor)))
  (머티리얼|GetBackMaterial _material_data)
  (Class|IPlaceableObject|DestroyObject(Message) (Variables|Building|GetDestroy%20Actor))
  (Variables|Building|SetDestroy%20Actor 0))

(fn RotateBuildingPrice
  (params (Axis%20Value :type Float%20%28double-precision%29))
  (LocalVariables|SetAction%20Value Axis%20Value)
  (if (Variables|Building|GetIsBuildMode)
    (Utilities|IsValid (Variables|Building|GetBuildinigPrice)
      (:Is%20Valid
        (if (Utilities|Array|IsValidIndex (Variables|Building|GetCheckCollisions))
          (Build|RotateCollision (LocalVariables|GetAction%20Value))
          (else
            (Build|RotateDegree (LocalVariables|GetAction%20Value))))))))

(fn CreateBuildPrice
  (bind _returnvalue (Utilities|LoadClassAssetBlocking (Class|KismetSystemLibrary|ToSoftClassRef(SoftClassPath) (Class|KismetSystemLibrary|MakeSoftClassPath (.classpath (Variables|Building|GetBuildPriceData))))))
  (bind _as액터 (Utilities|Casting|CastToActorClass _returnvalue))
  (bind _returnvalue_2 (Game|SpawnActorfromClass _as액터 (Math|Transform|MakeTransform (.location (Transformation|GetActorTransform (Variables|Components|GetPlayerPawn))) "0, 0, 0" "1.000000,1.000000,1.000000") "Undefined" 0 0))
  (bind _asbp_placeable_object_base (Utilities|Casting|CastToBP_PlaceableObjectBase _returnvalue_2))
  (Variables|Building|SetBuildinigPrice _asbp_placeable_object_base)
  (Variables|/Game/BuildingSystem/Blueprints/PlaceableObject/BP_PlaceableObjectBase.BP_PlaceableObjectBase_C|SetData (Variables|Building|GetBuildinigPrice) (Variables|Building|GetBuildPriceData)))

(fn InputInitialize
  (bind _playercont (Variables|Components|GetPlayerCont))
  (bind _returnvalue (PlayerController|LocalPlayerSubsystems|GetEnhancedInputLocalPlayerSubsystem _playercont))
  ;[1 1 1] IMC 등록
  (Utilities|IsValid (Variables|Components|GetPlayerCont)
    (:Is%20Valid
      (Utilities|IsValid _returnvalue
        (:Is%20Valid
          (Input|AddMappingContext _returnvalue "/Game/BuildingSystem/Input/IMC_Build.IMC_Build" 0 "(bIgnoreAllPressedKeysUntilRelease=True,bForceImmediately=False)"))
        (:Is%20Not%20Valid
          (Development|PrintString "Local Player Subsystem Not Valid" true true "(R=1.000000,G=0.000000,B=0.000000,A=1.000000)"))))
    (:Is%20Not%20Valid
      (Development|PrintString "Player Controller Not Valid" true true "(R=1.000000,G=0.000000,B=0.000000,A=1.000000)"))))

(fn Initialize
  (Initialize|ComponentsInitialize)
  (Initialize|InputInitialize)
  (Initialize|WidgetInitialize))

(fn ComponentsInitialize
  (bind _returnvalue (Game|GetPlayerCharacter 0))
  (bind _returnvalue_2 (Actor|GetComponentbyClass _returnvalue "/Game/BuildingSystem/Blueprints/Components/InventoryComponent.InventoryComponent_C"))
  ;[1 1 1] Player 관련 변수 설정
  (Variables|Components|SetPlayerCont (Game|GetPlayerController 0))
  (Variables|Components|SetPlayerPawn (Game|Player|GetPlayerPawn 0))
  (Utilities|IsValid _returnvalue_2
    (:Is%20Valid
      (Variables|컴포넌트|SetInventoryComp _returnvalue_2))))

(fn RotateDegree
  (params (Axis%20Value :type Float%20%28double-precision%29))
  (Transformation|SetActorRotation (Variables|Building|GetBuildinigPrice) (Math|Rotator|CombineRotators (Transformation|GetActorRotation (Variables|Building|GetBuildinigPrice)) (Math|Rotator|MakeRotator 0.0 0.0 (* Axis%20Value 1e+01)))))

(fn CheckforOverlap
  (bind _buildinigprice (Variables|Building|GetBuildinigPrice))
  (bind _returnvalue (Actor|GetComponentbyClass _buildinigprice "/Script/Engine.StaticMeshComponent"))
  (bind (_origin _boxextent) (Collision|GetComponentBounds _returnvalue))
  (bind _returnvalue_2 (Collision|BoxTraceByChannel _origin _origin (/ _boxextent 2.0) "0, 0, 0" "TraceTypeQuery1" false 0 "None"))
  (return _returnvalue_2))

(fn ClearBuildPrice
  (Utilities|IsValid (Variables|Building|GetBuildinigPrice)
    (:Is%20Valid
      (bind (_material_data _success) (Default|GetBackMaterials (Variables|Building|GetBuildinigPrice)))
      (if _success
        (머티리얼|GetBackMaterial _material_data))
      (Actor|DestroyActor (Variables|Building|GetBuildinigPrice))
      (CallFunction|ResetBuild))))

(fn RotateCollision
  (params (Axis%20Value :type Float%20%28double-precision%29))
  (if (>= Axis%20Value 0.0)
    (bind _result (Math|Integer|IncrementInt (Variables|Building|GetCheckCollisionIndex))
      (:%20%20
        (if (not (Utilities|Array|IsValidIndex (Variables|Building|GetCheckCollisions) _result))
          (Variables|Building|SetCheckCollisionIndex 0))))
    (else
      (bind _result_2 (Math|Integer|DecrementInt (Variables|Building|GetCheckCollisionIndex))
        (:%20%20
          (if (not (Utilities|Array|IsValidIndex (Variables|Building|GetCheckCollisions) _result_2))
            (Variables|Building|SetCheckCollisionIndex (- (Utilities|Array|Length (Variables|Building|GetCheckCollisions)) 1))))))))

(fn SetDestroyMode
  (params (Destroy%20Mode :type Boolean))
  (if Destroy%20Mode
    (Default|Close (Variables|Widgets|GetInventoryWidget)))
  (Variables|Building|SetIsDestroyMode Destroy%20Mode)
  (Class|IPlaceableObject|ChangeDefaultMaterial(Message) (Variables|Building|GetDestroy%20Actor)))

(fn Crafting
  (params (CraftingData :type Crafting%20Structure))
  (bind _success (Material|CheckMaterial (.materialid CraftingData)))
  (if _success
    (Default|AddItem (Variables|컴포넌트|GetInventoryComp) (.resultid CraftingData) (.resultcount CraftingData))))

(fn GetTraceLocation
  (bind _returnvalue (Game|GetPlayerCameraManager 0))
  (bind _transformcomponent (Variables|/Script/Engine.PlayerCameraManager|GetTransformComponent _returnvalue))
  (return (Transformation|GetActorLocation (Variables|Components|GetPlayerPawn)) (+ (Transformation|GetWorldLocation _transformcomponent) (* (Math|Vector|GetForwardVector _transformcomponent) 1e+04))))

(fn GetBuildTraceChannel
  (switch Utilities|FlowControl|Switch|SwitchonModelType (.typeid (Variables|Building|GetBuildPriceData))
    (:NewEnumerator0
      (return "TraceTypeQuery3"))
    (:NewEnumerator1
      (return "TraceTypeQuery4"))
    (:NewEnumerator2
      (return "TraceTypeQuery5"))
    (:NewEnumerator3
      (return "TraceTypeQuery6"))
    (:NewEnumerator4
      (return "TraceTypeQuery7"))))