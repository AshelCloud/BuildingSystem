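; Inventory component for the building system that tracks the local player's material counts in an enum-keyed map and mirrors them in a HUD widget.
; BeginPlay caches the player controller and pawn, adds an Enhanced Input mapping, seeds starting materials and creates the HUD.
; The pickup input passes the component to the first overlapping item's pickup message, then destroys the item.
; GetBackMaterial adds two material amounts back to the map and refreshes the HUD.
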(event Input|EnhancedActionEvents|EnhancedInputActionIA_Pickup
  (params (ActionValue :type Boolean) (ElapsedSeconds :type Float%20%28double-precision%29) (TriggeredSeconds :type Float%20%28double-precision%29) (InputAction :type Input%20Action%20Object%20Reference :default "/Game/BuildingSystem/Input/IA_Pickup.IA_Pickup"))
  (:Started
    (CallFunction|Pickup)))

(event EventBeginPlay
  (CallFunction|Initialize))

(fn InputInitialize
  (bind _playercont (Variables|Default|GetPlayerCont))
  (bind _returnvalue (PlayerController|LocalPlayerSubsystems|GetEnhancedInputLocalPlayerSubsystem _playercont))
  (Utilities|IsValid _returnvalue
    (:Is%20Valid
      (Input|AddMappingContext _returnvalue "/Game/BuildingSystem/Input/IMC_Inventory.IMC_Inventory" 0 "(bIgnoreAllPressedKeysUntilRelease=True,bForceImmediately=False)"))))

(fn ComponentInitialize
  (Variables|Default|SetPlayerCont (Game|GetPlayerController 0))
  (Variables|Default|SetPlayerPawn (Game|Player|GetPlayerPawn 0)))

(fn MaterialInitialize
  (Utilities|Map|Add (Variables|Default|GetMaterialMap) "NewEnumerator1" 100)
  (Utilities|Map|Add (Variables|Default|GetMaterialMap) "NewEnumerator2" 100))

(fn Pickup
  (bind _actor (CallFunction|OverlapCheck))
  (LocalVariables|SetPick%20Actor _actor)
  (Utilities|IsValid (LocalVariables|GetPick%20Actor)
    (:Is%20Valid
      (Class|IPickupObject|Pickup(Message) (LocalVariables|GetPick%20Actor) self)
      (Actor|DestroyActor (LocalVariables|GetPick%20Actor))
      (CallFunction|UpdateHUD))))

(fn Initialize
  (Initialize|ComponentInitialize)
  (Initialize|InputInitialize)
  (Initialize|MaterialInitialize)
  (CallFunction|CreateHUD))

(fn OverlapCheck
  (return (Utilities|Array|Get(acopy) (Collision|GetOverlappingActors (Variables|Default|GetPlayerPawn) "/Game/BuildingSystem/Blueprints/Item/BP_ItemBase.BP_ItemBase_C" :!class /Script/Engine.Actor))))

(fn CreateHUD
  (bind _returnvalue (UserInterface|CreateWidget "/Game/BuildingSystem/Blueprints/UserInterface/WBP_HUD.WBP_HUD_C"))
  (Variables|Default|SetHUD _returnvalue)
  (Default|Initialize _returnvalue (Variables|Default|GetMaterialMap))
  (UserInterface|Viewport|AddtoViewport _returnvalue 0))

(fn UpdateHUD
  (Default|UpdateText (Variables|Default|GetHUD) (Variables|Default|GetMaterialMap)))

(fn GetBackMaterial
  (params (Data :type Build%20Material%20Structure))
  (LocalVariables|SetLocal%20Data Data)
  (Utilities|FlowControl|Sequence
    (:then_0
      (if (.ReturnValue (Utilities|Map|Find (Variables|Default|GetMaterialMap) (.Material_1_Type (Utilities|Struct|BreakBuildMaterial (LocalVariables|GetLocal%20Data)))))
        (Utilities|Map|Add (Variables|Default|GetMaterialMap) (.Material_1_Type (Utilities|Struct|BreakBuildMaterial (LocalVariables|GetLocal%20Data))) (+ (.Value (Utilities|Map|Find (Variables|Default|GetMaterialMap) (.Material_1_Type (Utilities|Struct|BreakBuildMaterial (LocalVariables|GetLocal%20Data))))) (.Material_1_Count (Utilities|Struct|BreakBuildMaterial (LocalVariables|GetLocal%20Data)))))))
    (:then_1
      (if (.ReturnValue (Utilities|Map|Find (Variables|Default|GetMaterialMap) (.Material_2_Type (Utilities|Struct|BreakBuildMaterial (LocalVariables|GetLocal%20Data)))))
        (Utilities|Map|Add (Variables|Default|GetMaterialMap) (.Material_2_Type (Utilities|Struct|BreakBuildMaterial (LocalVariables|GetLocal%20Data))) (+ (.Value (Utilities|Map|Find (Variables|Default|GetMaterialMap) (.Material_2_Type (Utilities|Struct|BreakBuildMaterial (LocalVariables|GetLocal%20Data))))) (.Material_2_Count (Utilities|Struct|BreakBuildMaterial (LocalVariables|GetLocal%20Data)))))))
    (:then_2
      (CallFunction|UpdateHUD))))