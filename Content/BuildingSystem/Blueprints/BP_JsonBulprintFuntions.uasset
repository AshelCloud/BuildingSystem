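; BP_JsonBulprintFuntions provides helper functions that load building system data tables from JSON files.
; ReadJson loads a named file from the project's Content/Jsons folder and reports success.
; Two readers build on it, extracting the "data" field from the build model and material tables.
; The material reader linearly searches for a matching ID and returns a BuildMaterial struct with two material type and count pairs.
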(fn ReadJson
  (params (TableName :type String))
  (bind (_outjsonobject _returnvalue) (Class|JsonBlueprintFunctionLibrary|FromFile (Utilities|Struct|MakeFilePath (Utilities|String|Append (Class|KismetSystemLibrary|GetProjectContentDirectory) "Jsons/" TableName))))
  (return _outjsonobject _returnvalue))

(fn ReadBuildModelJson
  (bind (_json _success) (CallFunction|ReadJson "BuildModelTable.json"))
  (if _success
    (bind (_outvalue _returnvalue) (|GetJsonField _json "data"))
    (return _outvalue _returnvalue)))

(fn ReadMaterialJsonwithTypeID
  (params (ID :type Integer))
  (LocalVariables|SetResultID ID)
  (bind (_json _success) (CallFunction|ReadJson "MaterialTable.json"))
  (if _success
    (bind (_outvalue _returnvalue) (|GetJsonField _json "data"))
    (for _array_element _outvalue
      (if (== (LocalVariables|GetResultID) (.ID (Utilities|Struct|BreakBuildMaterial _array_element)))
        (return (Utilities|Struct|MakeBuildMaterial (.ID (Utilities|Struct|BreakBuildMaterial _array_element)) (.Material_1_Type (Utilities|Struct|BreakBuildMaterial _array_element)) (.Material_1_Count (Utilities|Struct|BreakBuildMaterial _array_element)) (.Material_2_Type (Utilities|Struct|BreakBuildMaterial _array_element)) (.Material_2_Count (Utilities|Struct|BreakBuildMaterial _array_element))) _returnvalue)))))